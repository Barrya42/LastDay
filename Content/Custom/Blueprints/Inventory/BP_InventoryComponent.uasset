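; Inventory component that stores picked-up drops in an array of slot structs and uses them for the top-down player character.
; AddDrop searches for a matching Id to stack onto, otherwise appends the drop while below MaxItems, printing slot contents for debugging.
; AddCountToItem is an empty stub with its count and weight update disconnected, so stacking changes nothing.
; InventoryClicked sends UseDropMessage to the slot's referenced actor, passing the character cached at BeginPlay.
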(event Custom|InventoryClicked
  (params (InventorySlot :type Integer))
  ;[1 1 1] Исползуем инвентарь(НУЖЕН ЛИ ТАКОЙ КРЮК ЧЕРЕЗ КОМПОНЕНТУ!!!!)
  (Class|UsableDrop|UseDrop(Message) (.ActorReference (Utilities|Struct|BreakS_InventorySlotStruct (Utilities|Array|Get(acopy) (Variables|DropStruct|GetInventory) InventorySlot))) (Variables|Default|GetCharacter)))

(event EventBeginPlay
  (bind _astop_down_character (Utilities|Casting|CastToTopDownCharacter (Game|GetPlayerCharacter 0)))
  (Variables|Default|SetCharacter _astop_down_character))

(fn AddDrop
  (params (Drop :type S%20Inventory%20Slot%20Struct%20Structure))
  (bind _output_get (LocalVariables|SetL_Drop Drop))
  (bind (_index _value _founded) (Drop|SearchinInventory _output_get))
  (if _founded
    (Drop|AddCounttoItem _index (.count (LocalVariables|GetL_Drop)) (.weight (LocalVariables|GetL_Drop)))
    (for (_array_element _array_index) (Variables|DropStruct|GetInventory)
      (Development|PrintString (Utilities|String|Append (Utilities|String|Append (Utilities|String|ToString(Integer) (+ _array_index 1)) (Utilities|String|ToString(Text) (.Name (Utilities|Struct|BreakS_InventorySlotStruct _array_element)))) (Utilities|String|ToString(Float) (.Count (Utilities|Struct|BreakS_InventorySlotStruct _array_element))))))
    (elif (< (Utilities|Array|Length (Variables|DropStruct|GetInventory)) (Variables|Default|GetMaxItems))
      (Utilities|Array|Add (Variables|DropStruct|GetInventory) (LocalVariables|GetL_Drop))
      (Development|PrintString (Utilities|String|Append (Utilities|String|Append (Utilities|String|ToString(Integer) (+ _array_index 1)) (Utilities|String|ToString(Text) (.Name (Utilities|Struct|BreakS_InventorySlotStruct _array_element)))) (Utilities|String|ToString(Float) (.Count (Utilities|Struct|BreakS_InventorySlotStruct _array_element))))))))

(fn SearchinInventory
  (params (Drop :type S%20Inventory%20Slot%20Struct%20Structure))
  (LocalVariables|SetL_Drop Drop)
  (bind (_array_element _array_index) (Utilities|Array|ForEachLoopwithBreak (Variables|DropStruct|GetInventory) :!label _label)
    (:LoopBody
      (if (== (.Id (Utilities|Struct|BreakS_InventorySlotStruct _array_element)) (.Id (Utilities|Struct|BreakS_InventorySlotStruct (LocalVariables|GetL_Drop))))
        (LocalVariables|SetCurentIndex _array_index)
        (LocalVariables|SetL_Founded true)
        (goto _label Break)))
    (:Completed
      (return (LocalVariables|GetCurentIndex) _array_element (LocalVariables|GetL_Founded)))))

(fn AddCounttoItem
  (params (Item :type Integer) (Count :type Float%20%28single-precision%29) (Weight :type Float%20%28single-precision%29)))