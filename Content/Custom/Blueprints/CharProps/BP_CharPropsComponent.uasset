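; Character stats component that manages health and energy, with damage, healing, spending and regeneration.
; Tick runs health regen, energy change and energy regen each frame, with optional on-screen debug readouts.
; ChangeEnergy either drains over time or applies a one-off delta clamped to valid bounds, while health changes are not clamped.
; Changes broadcast HealthChanged and EnergyChanged, except timed energy drain, and SwitchEnergyRegen toggles energy regen.
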(event EventBeginPlay)

(event EventTick
  (params (DeltaSeconds :type Float%20%28single-precision%29))
  (Utilities|FlowControl|Sequence
    (:then_0
      (Health|RegenHealth 0.0)
      (Energy|ChangeEnergy (Variables|Energy|GetUseEnegrySpend) 0.0)
      (Energy|RegenEnegry 0.0))
    (:then_1
      (if (Variables|Default|GetShowDebug)
        (Development|PrintString (Utilities|String|Append "Health: " (Utilities|String|ToString(Float) (Variables|Health|GetHealth))) true false "(R=0.000000,G=1.000000,B=0.038341,A=1.000000)" 0.0)
        (Development|PrintString (Utilities|String|Append "Energy: " (Utilities|String|ToString(Float) (Variables|Energy|GetEnergy))) true false "(R=1.000000,G=0.829904,B=0.000000,A=1.000000)" 0.0)))))

(fn RegenHealth
  (params (AdditionalRegen :type Float%20%28single-precision%29))
  ;[1 1 1] Regeneration
  (LocalVariables|SetL_AdditionalRegen AdditionalRegen)
  (if (and (Variables|Health|GetUseHealthRegeniration) (< (Variables|Health|GetHealth) (Variables|Health|GetMaxHealth)))
    (bind _output_get (Variables|Health|SetHealth (+ (Variables|Health|GetHealth) (* (+ (LocalVariables|GetL_AdditionalRegen) (Variables|Health|GetHealthRegenSpeed)) (Utilities|Time|GetWorldDeltaSeconds)))))
    (Default|CallHealthChanged _output_get)))

(fn Heal
  (params (Heal :type Float%20%28single-precision%29))
  (LocalVariables|SetL_Heal Heal)
  (if (< (Variables|Health|GetHealth) (Variables|Health|GetMaxHealth))
    (bind _output_get (Variables|Health|SetHealth (+ (LocalVariables|GetL_Heal) (Variables|Health|GetHealth))))
    (Default|CallHealthChanged _output_get)))

(fn Damage
  (params (Damage :type Float%20%28single-precision%29))
  (LocalVariables|SetL_Damage Damage)
  (if (> (Variables|Health|GetHealth) 0.0)
    (bind _output_get (Variables|Health|SetHealth (- (Variables|Health|GetHealth) (LocalVariables|GetL_Damage))))
    (Default|CallHealthChanged _output_get)))

(fn ChangeEnergy
  (params (IsSpending :type Boolean) (EnergyChangeForSomeAction :type Float%20%28single-precision%29))
  (Utilities|FlowControl|Sequence
    (:then_0
      (LocalVariables|SetL_AnergyForSomeAction EnergyChangeForSomeAction)
      (LocalVariables|SetL_IsSpending IsSpending))
    (:then_1
      ;[1 1 1] SpendEnergyWithTime
      (if (LocalVariables|GetL_IsSpending)
        (if (>= (- (Variables|Energy|GetEnergy) (* (Variables|Energy|GetEnergySpendSpeed) (Utilities|Time|GetWorldDeltaSeconds))) 0.0)
          (Variables|Energy|SetEnergy (- (Variables|Energy|GetEnergy) (* (Variables|Energy|GetEnergySpendSpeed) (Utilities|Time|GetWorldDeltaSeconds))))
          (else
            (Variables|Energy|SetEnergy 0.0)))
        (else
          ;[1 1 1] ChangeEnegryWithReason
          (if (< (LocalVariables|GetL_AnergyForSomeAction) 0.0)
            ;;[1 1 1] Уменьшим энергию
            (if (> (+ (Variables|Energy|GetEnergy) (LocalVariables|GetL_AnergyForSomeAction)) 0.0)
              (Variables|Energy|SetEnergy (+ (Variables|Energy|GetEnergy) (LocalVariables|GetL_AnergyForSomeAction)))
              (else
                (bind _output_get (Variables|Energy|SetEnergy 0.0))))
            (Default|CallEnergyChanged _output_get)
            (else
              ;;[1 1 1] Увеличим
              (bind _output_get_2 (Variables|Energy|SetEnergy (Math|Float|Clamp(Float) (+ (Variables|Energy|GetEnergy) (LocalVariables|GetL_AnergyForSomeAction)) 0.0 (Variables|Energy|GetMaxEnergy))))
              (Default|CallEnergyChanged _output_get_2))))))))

(fn RegenEnegry
  (params (AdditionalRegen :type Float%20%28single-precision%29))
  ;[1 1 1] Regeneration
  (LocalVariables|SetL_AdditionalRegen AdditionalRegen)
  (if (Math|Boolean|ANDBoolean (Variables|Energy|GetEnergyRegenIsOn) (Variables|Energy|GetUseEnergyRegeniration) (< (Variables|Energy|GetEnergy) (Variables|Energy|GetMaxEnergy)))
    (bind _output_get (Variables|Energy|SetEnergy (+ (Variables|Energy|GetEnergy) (* (+ (LocalVariables|GetL_AdditionalRegen) (Variables|Energy|GetEnergyRegenSpeed)) (Utilities|Time|GetWorldDeltaSeconds)))))
    (Default|CallEnergyChanged _output_get)))

(fn SwitchEnergyRegen
  (params (Value :type Boolean))
  (Variables|Energy|SetEnergyRegenIsOn Value))